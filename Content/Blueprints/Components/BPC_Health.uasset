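; Health component that holds a clamped current health value, with functions to add and remove health.
; UpdateHealth routes positive changes to AddHealth, printing the result, and passes other changes unnegated to RemoveHealth, which subtracts them, so negative inputs raise health.
; RemoveHealth's alive check is inverted: IsAlive is true at or below minimum, and otherwise false with zero returned as health, which UpdateHealth stores.
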(event EventBeginPlay)

(event EventTick
  (params (DeltaSeconds :type Float%20%28single-precision%29)))

(fn RemoveHealth
  (params (Damage :type Float%20%28double-precision%29))
  (bind _output_get (Variables|Health|SetCurrentHealth (Math|Float|Clamp(Float) (- (Variables|Health|GetCurrentHealth) Damage) (Variables|Health|GetMinHealth) (Variables|Health|GetMaxHealth))))
  ;[1 1 1] Check is player alive and is the player above 0
  (if (<= (Variables|Health|GetCurrentHealth) (Variables|Health|GetMinHealth))
    (bind _output_get_2 (Variables|Default|SetisAlive true))
    ;;[1 1 1] check this
    (return _output_get _output_get_2)
    (else
      (bind _output_get_3 (Variables|Default|SetisAlive false))
      (return 0.0 _output_get_3))))

(fn AddHealth
  (params (AmountAdd :type Float%20%28double-precision%29))
  (bind _output_get (Variables|Health|SetCurrentHealth (Math|Float|Clamp(Float) (+ (Variables|Health|GetCurrentHealth) AmountAdd) (Variables|Health|GetMinHealth) (Variables|Health|GetMaxHealth))))
  (return _output_get))

(fn UpdateHealth
  (params (HealthAmountChange :type Float%20%28double-precision%29))
  (if (> HealthAmountChange 0.0)
    (bind _health (CallFunction|AddHealth HealthAmountChange))
    (bind _output_get (Variables|Health|SetCurrentHealth _health))
    (Development|PrintString (Utilities|String|ToString(Float) (Variables|Health|GetCurrentHealth)) true true "(R=0.000000,G=0.660000,B=1.000000,A=1.000000)" 5.0)
    (return _output_get)
    (else
      (bind _health_2 (CallFunction|RemoveHealth HealthAmountChange))
      (bind _output_get_2 (Variables|Health|SetCurrentHealth _health_2))
      (return _output_get_2))))