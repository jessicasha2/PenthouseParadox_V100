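; Master hide spot actor that hides BP_MysteryChar when the character overlaps its box.
; Begin overlap caches the character, enables its input and toggles on IsHiding between UnHideChar and HideChar.
; Hiding blends the player's view to this actor, then after a short delay loops back into that same check.
; End overlap disables input, then also jumps into the hide branch.
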(event OnComponentBeginOverlap(Box)
  (params (OverlappedComponent :type Primitive%20Component%20Object%20Reference) (OtherActor :type Actor%20Object%20Reference) (OtherComp :type Primitive%20Component%20Object%20Reference) (OtherBodyIndex :type Integer) (bFromSweep :type Boolean) (SweepResult :type Hit%20Result%20Structure%20%28by%20ref%29))
  (bind _asbp_mystery_char (Utilities|Casting|CastToBP_MysteryChar OtherActor))
  (bind _output_get (Variables|Default|SetCharacter%20REF _asbp_mystery_char))
  (Input|EnableInput _output_get (Game|GetPlayerController 0) :!label _label)
  (if (Variables|/Game/Blueprints/GAME/BP_MysteryChar.BP_MysteryChar_C|GetisHiding? (Variables|Default|GetCharacter%20REF))
    (Default|UnHideChar (Variables|Default|GetCharacter%20REF))
    (else
      (Default|HideChar (Variables|Default|GetCharacter%20REF))
      (Utilities|FlowControl|Sequence
        (:then_0
          (Game|Player|SetViewTargetwithBlend (Game|GetPlayerController 0) self 0.5 "VTBlend_Linear" 0.0 false))
        (:then_1
          (Utilities|FlowControl|Delay 0.2)
          (goto _label))))))

(event OnComponentEndOverlap(Box)
  (params (OverlappedComponent :type Primitive%20Component%20Object%20Reference) (OtherActor :type Actor%20Object%20Reference) (OtherComp :type Primitive%20Component%20Object%20Reference) (OtherBodyIndex :type Integer))
  (bind _returnvalue (Game|GetPlayerController 0))
  (bind _character_ref (Variables|Default|GetCharacter%20REF))
  (Utilities|Casting|CastToBP_MysteryChar OtherActor)
  (Input|DisableInput (stale OnComponentBeginOverlap(Box) _output_get) _returnvalue)
  (Default|HideChar _character_ref :!label _label)
  (Utilities|FlowControl|Sequence
    (:then_0
      (Game|Player|SetViewTargetwithBlend (Game|GetPlayerController 0) self 0.5 "VTBlend_Linear" 0.0 false))
    (:then_1
      (Utilities|FlowControl|Delay 0.2)
      (Input|EnableInput (stale OnComponentBeginOverlap(Box) _output_get) _returnvalue)
      (if (Variables|/Game/Blueprints/GAME/BP_MysteryChar.BP_MysteryChar_C|GetisHiding? (Variables|Default|GetCharacter%20REF))
        (Default|UnHideChar _character_ref)
        (else
          (goto _label))))))

(event EventBeginPlay)

(event Collision|EventActorBeginOverlap
  (params (OtherActor :type Actor%20Object%20Reference)))

(event EventTick
  (params (DeltaSeconds :type Float%20%28single-precision%29)))

(fn ConstructionScript)